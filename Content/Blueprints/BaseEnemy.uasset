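; Base enemy character that chases the player pawn with AIMoveTo issued every Tick while not stunned.
; Capsule hits on a Doll knock the player back, then pause the enemy briefly.
; Knockback stuns it, subtracts the Doll's PlayerSTR from EnemyHealth, then destroys it or launches it along the Doll's ForwardVector.
; Blocked stuns it with a zero-velocity launch; all pauses share the EnemyStunned flag, cleared after delays.
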(event OnComponentHit(CapsuleComponent)
  (params (HitComponent :type Primitive%20Component%20Object%20Reference) (OtherActor :type Actor%20Object%20Reference) (OtherComp :type Primitive%20Component%20Object%20Reference) (NormalImpulse :type Vector :default "0, 0, 0") (Hit :type Hit%20Result%20Structure%20%28by%20ref%29))
  ;[0 1 0.04932 0.2] ATTACK
  (bind _asdoll (Utilities|Casting|CastToDoll OtherActor))
  (Default|PlayerKnockback _asdoll (Transformation|GetActorForwardVector))
  (CallFunction|Cooldown))

(event Custom|Stunned
  ;[0 1 0.108 0.2] STUNNED (PAUSE FROM KNOCKBACK)
  (Variables|Default|SetEnemyStunned true)
  (Components|Movement|StopMovementImmediately (Variables|Character|GetCharacterMovement))
  (Utilities|FlowControl|Delay 2.0)
  (Variables|Default|SetEnemyStunned false))

(event Custom|Cooldown
  ;[0 1 0.09921 0.2] COOLDOWN (PAUSE AFTER ATTACKING PLAYER)
  (Variables|Default|SetEnemyStunned true)
  (Components|Movement|StopMovementImmediately (Variables|Character|GetCharacterMovement))
  (Utilities|FlowControl|Delay 1.0)
  (Variables|Default|SetEnemyStunned false))

(event Custom|Knockback
  ;[0 1 0.1462 0.2] KNOCKBACK
  (CallFunction|Stunned)
  (bind _asdoll (Utilities|Casting|CastToDoll (Game|Player|GetPlayerPawn 0)))
  (Variables|Default|SetEnemyHealth (- (Variables|Default|GetEnemyHealth) (Variables|/Game/Blueprints/Doll.Doll_C|GetPlayerSTR _asdoll)))
  (if (<= (Variables|Default|GetEnemyHealth) 0)
    (Actor|DestroyActor)
    (Variables|Default|SetDead true)
    (else
      (Character|LaunchCharacter (* (Variables|/Game/Blueprints/Doll.Doll_C|GetForwardVector _asdoll) "1000.000000,1000.000000,1000.000000") false false)
      (Variables|Default|SetDead false))))

(event Custom|Blocked
  (CallFunction|Stunned)
  (Character|LaunchCharacter (* "" "1000.000000,1000.000000,1000.000000") false false))

(event EventTick
  (params (DeltaSeconds :type Float%20%28single-precision%29))
  ;[0.02376 1 0 0.2] ENEMY MOVEMENT
  (if (not (Variables|Default|GetEnemyStunned))
    (AI|AIMoveTo self "0, 0, 0" (Game|Player|GetPlayerPawn 0) 1e+01 false)))

(fn ConstructionScript)